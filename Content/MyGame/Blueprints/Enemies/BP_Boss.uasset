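; Boss enemy that chases the player, attacks and dies with a montage before being destroyed, under a camera-facing health bar.
; Pawn sensing sets a blackboard chase flag on sighting the third-person character.
; AttackPlayer randomly plays one of two montages, one also spawning BP_BossAtk, and re-arms after a delay.
; The hand collider damages the player, while player skill projectiles deal heavier damage on the back collider than on the capsule.
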(event OnComponentBeginOverlap(HandCollider)
  (params (OverlappedComponent :type Primitive%20Component%20Object%20Reference) (OtherActor :type Actor%20Object%20Reference) (OtherComp :type Primitive%20Component%20Object%20Reference) (OtherBodyIndex :type Integer) (bFromSweep :type Boolean) (SweepResult :type Hit%20Result%20Structure%20%28by%20ref%29))
  ;[1 1 1] Damage Player
  (bind _asbp_player (Utilities|Casting|CastToBP_Player OtherActor))
  (Class|BPIDamage|TakeDamage(Message) _asbp_player (Variables|EnemyStats|GetEnemyDamage)))

(event OnSeePawn(PawnSensing)
  (params (Pawn :type Pawn%20Object%20Reference))
  ;[1 1 1] Enemy AI
  (Utilities|Casting|CastToBP_ThirdPersonCharacter Pawn)
  (AI|Components|Blackboard|SetValueasBool (AI|GetBlackboard (AI|GetAIController self)) (Utilities|Name|MakeLiteralName "ChasingPlayer?") true))

(event OnComponentBeginOverlap(BackCollider)
  (params (OverlappedComponent :type Primitive%20Component%20Object%20Reference) (OtherActor :type Actor%20Object%20Reference) (OtherComp :type Primitive%20Component%20Object%20Reference) (OtherBodyIndex :type Integer) (bFromSweep :type Boolean) (SweepResult :type Hit%20Result%20Structure%20%28by%20ref%29))
  (Utilities|Casting|CastToBP_PlayerSkill1 OtherActor)
  (CallFunction|TakeDamage 80)
  (Actor|DestroyActor OtherActor))

(event OnComponentBeginOverlap(CapsuleComponent)
  (params (OverlappedComponent :type Primitive%20Component%20Object%20Reference) (OtherActor :type Actor%20Object%20Reference) (OtherComp :type Primitive%20Component%20Object%20Reference) (OtherBodyIndex :type Integer) (bFromSweep :type Boolean) (SweepResult :type Hit%20Result%20Structure%20%28by%20ref%29))
  (Utilities|Casting|CastToBP_PlayerSkill1 OtherActor)
  (CallFunction|TakeDamage 20)
  (Actor|DestroyActor OtherActor))

(event Custom|AttackPlayer
  ;[1 1 1] Enemy Attack Logic
  (bind (_returnvalue _particlesystem) (CallFunction|AttackAnim))
  (Utilities|FlowControl|Delay _returnvalue)
  (if (Utilities|IsValid _particlesystem)
    (Components|DestroyComponent _particlesystem))
  (Variables|Default|SetcanAttack? true))

(event EventBeginPlay
  ;[1 1 1] Initialize Variables
  (Variables|/Script/Engine.CharacterMovementComponent|SetMaxWalkSpeed (Variables|Character|GetCharacterMovement) (Variables|Animation|GetMovementSpeed))
  (Variables|EnemyStats|SetMaxHealth (Variables|EnemyStats|GetEnemyHP)))

(event EventTick
  (params (DeltaSeconds :type Float%20%28single-precision%29))
  ;[1 1 1] Health UI Update
  (bind _aswb_health_bar (Utilities|Casting|CastToWB_HealthBar (UserInterface|GetWidget (Variables|Default|GetHealthBar))))
  (Progress|SetPercent (Variables|/Game/MyGame/UI/WB_HealthBar.WB_HealthBar_C|GetHealth _aswb_health_bar) (/ (Variables|EnemyStats|GetEnemyHP) (Variables|EnemyStats|GetMaxHealth)))
  (Transformation|SetWorldRotation (Variables|Default|GetHealthBar) (Math|Rotator|FindLookatRotation (Transformation|GetWorldLocation (Variables|Default|GetHealthBar)) (Transformation|GetWorldLocation (Variables|/Script/Engine.PlayerCameraManager|GetTransformComponent (Game|GetPlayerCameraManager 0)))) false false))

(event EventTakeDamage
  (params (Damage :type Integer))
  ;[1 1 1] Take Damage
  (bind _output_get (Variables|EnemyStats|SetEnemyHP (- (Variables|EnemyStats|GetEnemyHP) Damage)))
  (if (<= _output_get 0)
    (bind _returnvalue (Animation|PlayAnimMontage (Variables|Animation|GetDeathMontage) 1.0 "None"))
    (Utilities|FlowControl|Delay _returnvalue)
    (Actor|DestroyActor)))

(fn ConstructionScript)

(fn AttackAnim
  (if (Variables|Default|GetcanAttack?)
    (Variables|Default|SetcanAttack? false)
    (if (== (Math|Integer|%(Integer) (Math|Random|RandomIntegerinRange 1 3) 2) 0)
      (Game|SpawnActorfromClass "/Game/MyGame/VFX/BP_BossAtk.BP_BossAtk_C" (Transformation|GetWorldTransform (Variables|Default|GetArrow1)) "AlwaysSpawn" "MultiplyWithRoot" 0 0)
      (bind _returnvalue (Animation|PlayAnimMontage (Variables|Default|GetAttackMontage2) 1.0 "None"))
      (return _returnvalue 0)
      (else
        (bind _returnvalue_2 (Animation|PlayAnimMontage (Variables|Default|GetAttackMontage1) 1.0 "None"))
        (return _returnvalue_2 0)))))