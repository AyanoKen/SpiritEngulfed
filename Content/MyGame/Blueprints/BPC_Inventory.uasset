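; Inventory component that stores picked-up items in a five-slot array and shows them in a WB_Inventory widget toggled with the I key.
; Pressing E sphere-traces around the player's feet for a BP_BlackGear actor.
; One pass over the slots stacks it on a matching stackable item or fills an empty slot, whichever comes first.
; A successful pickup reloads the widget, destroys the actor and plays a sound.
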(event EventBeginPlay
  (bind _returnvalue (UserInterface|CreateWidget "/Game/MyGame/Inventory/Widgets/WB_Inventory.WB_Inventory_C"))
  (Variables|Default|SetInventoryWidget _returnvalue)
  (Utilities|Array|Resize (Variables|Default|GetItems) 5)
  (Default|LoadInventory (Variables|Default|GetInventoryWidget) self))

(event Input|KeyboardEvents|I
  (params (Key :type Key%20Structure :default "None"))
  (:Pressed
    (if (Widget|IsVisible (Variables|Default|GetInventoryWidget))
      (Widget|RemovefromParent (Variables|Default|GetInventoryWidget))
      (else
        (UserInterface|Viewport|AddtoViewport (Variables|Default|GetInventoryWidget) 0)))))

(event Input|KeyboardEvents|E
  (params (Key :type Key%20Structure :default "None"))
  (bind _returnvalue (Game|GetPlayerCharacter 0))
  (bind _returnvalue_2 (Transformation|GetActorLocation _returnvalue))
  (bind _returnvalue_3 (- _returnvalue_2 "0.000000,0.000000,65.000000"))
  (:Pressed
    (bind _outhit (Collision|SphereTraceByChannel _returnvalue_3 _returnvalue_3 1.2e+02 "TraceTypeQuery1" false 0 "None"))
    (bind _asbp_black_gear (Utilities|Casting|CastToBP_BlackGear (.HitActor (Collision|BreakHitResult _outhit))))
    (for (_array_element _array_index) (Variables|Default|GetItems)
      (Utilities|IsValid _asbp_black_gear
        (:Is%20Valid
          (if (and (Utilities|Enum|Equal(Enum) (.Name (Utilities|Struct|BreakS_Inventory _array_element)) (.Name (Utilities|Struct|BreakS_Inventory (Variables|/Game/MyGame/Blueprints/Collectables/BP_BlackGear.BP_BlackGear_C|GetItemInfo _asbp_black_gear)))) (.Stackable (Utilities|Struct|BreakS_Inventory (Variables|/Game/MyGame/Blueprints/Collectables/BP_BlackGear.BP_BlackGear_C|GetItemInfo _asbp_black_gear))))
            (Utilities|Array|SetArrayElem (Variables|Default|GetItems) _array_index (Utilities|Struct|MakeS_Inventory (.Name (Utilities|Struct|BreakS_Inventory (Variables|/Game/MyGame/Blueprints/Collectables/BP_BlackGear.BP_BlackGear_C|GetItemInfo _asbp_black_gear))) (.Stackable (Utilities|Struct|BreakS_Inventory (Variables|/Game/MyGame/Blueprints/Collectables/BP_BlackGear.BP_BlackGear_C|GetItemInfo _asbp_black_gear))) (+ (.Quantity (Utilities|Struct|BreakS_Inventory _array_element)) (.Quantity (Utilities|Struct|BreakS_Inventory (Variables|/Game/MyGame/Blueprints/Collectables/BP_BlackGear.BP_BlackGear_C|GetItemInfo _asbp_black_gear)))) (.ThumbNail (Utilities|Struct|BreakS_Inventory (Variables|/Game/MyGame/Blueprints/Collectables/BP_BlackGear.BP_BlackGear_C|GetItemInfo _asbp_black_gear))) (.mesh (Utilities|Struct|BreakS_Inventory (Variables|/Game/MyGame/Blueprints/Collectables/BP_BlackGear.BP_BlackGear_C|GetItemInfo _asbp_black_gear)))))
            (Default|LoadInventory (Variables|Default|GetInventoryWidget) self :!label _label)
            (Actor|DestroyActor _asbp_black_gear)
            (Audio|PlaySound2D "/Game/MyGame/SFX/ItemPickup_Cue.ItemPickup_Cue" 1.0 1.0 0.0 0 0)
            (elif (== (.Quantity (Utilities|Struct|BreakS_Inventory _array_element)) 0)
              (Utilities|Array|SetArrayElem (Variables|Default|GetItems) _array_index (Variables|/Game/MyGame/Blueprints/Collectables/BP_BlackGear.BP_BlackGear_C|GetItemInfo _asbp_black_gear))
              (goto _label))))))))