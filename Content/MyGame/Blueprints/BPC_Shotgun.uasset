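; Shotgun weapon actor that implements the WeaponTrace event to fire a multi-pellet hitscan blast from the player camera.
; Each pellet is a thin sphere trace on the Visibility channel, randomised within a cone set by WeaponSpread.
; Every pellet hitting an actor that implements BPI_Damage sends it WeaponDamage through TakeDamage, so damage stacks per pellet.
; Traces leave persistent debug drawing.
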(event EventBeginPlay
  (|CallParentFunction) ; This node is disabled and will not be called.\nDrag off pins to build functionality.
)

(event Collision|EventActorBeginOverlap
  (params (OtherActor :type Actor%20Object%20Reference))
  (|CallParentFunction OtherActor) ; This node is disabled and will not be called.\nDrag off pins to build functionality.
)

(event EventTick
  (params (DeltaSeconds :type Float%20%28single-precision%29))
  (|CallParentFunction DeltaSeconds) ; This node is disabled and will not be called.\nDrag off pins to build functionality.
)

(event EventWeaponTrace
  (bind _returnvalue (Game|GetPlayerCameraManager 0))
  (bind _transformcomponent (Variables|/Script/Engine.PlayerCameraManager|GetTransformComponent _returnvalue))
  (bind _returnvalue_2 (Transformation|GetWorldLocation _transformcomponent))
  (for _index (range 0 9)
    (bind _outhit (Collision|SphereTraceByChannel _returnvalue_2 (+ (* (Math|Random|RandomUnitVectorinConeinDegrees (Math|Vector|GetForwardVector _transformcomponent) (Variables|Default|GetWeaponSpread)) 3e+03) _returnvalue_2) 1.0 "TraceTypeQuery1" false 0 "Persistent"))
    (if (Utilities|DoesObjectImplementInterface (.HitActor (Collision|BreakHitResult _outhit)) "/Game/MyGame/Blueprints/BPI_Damage.BPI_Damage_C")
      (Class|BPIDamage|TakeDamage(Message) (.HitActor (Collision|BreakHitResult _outhit)) (Variables|Default|GetWeaponDamage)))))

(fn ConstructionScript
  (|CallParentFunction))