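; Old man NPC that gives a plant-collection quest and drives its dialogue and HUD quest text.
; EventIndex tracks quest stage, with Tick polling the player's inventory during stage 1 for ten BlackGear items.
; StartDialogue opens the widget and locks movement, then steps through lines on repeat calls, which only stages 0 and 2 handle.
; Finishing dialogue restores movement and advances the quest, ending on a season-complete message.
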(event EventTick
  (params (DeltaSeconds :type Float%20%28single-precision%29))
  (if (== (Variables|Default|GetEventIndex) 1)
    (bind _asbp_player (Utilities|Casting|CastToBP_Player (Game|Player|GetPlayerPawn 0)))
    (for _array_element (Variables|/Game/MyGame/Blueprints/BPC_Inventory.BPC_Inventory_C|GetItems (Variables|/Game/MyGame/Blueprints/BP_Player.BP_Player_C|GetBPC_Inventory _asbp_player))
      (if (Utilities|Enum|Equal(Enum) (.Name (Utilities|Struct|BreakS_Inventory _array_element)) (Utilities|Text|MakeLiteralText "BlackGear"))
        (if (>= (.Quantity (Utilities|Struct|BreakS_Inventory _array_element)) 10)
          (Math|Integer|IncrementInt (Variables|Default|GetEventIndex)
            (:%20%20
              (bind _asmy_hud (Utilities|Casting|CastToMyHUD (HUD|GetHUD (Game|GetPlayerController 0))))
              (Variables|/Script/UMG.TextBlock|SetText (Variables|/Game/MyGame/UI/WB_UI.WB_UI_C|GetQuest1 (Variables|/Game/MyGame/UI/MyHUD.MyHUD_C|GetUI_Ref _asmy_hud)) "Collect the plants the mysterious man asked for (10/10)")
              (Variables|/Script/UMG.TextBlock|SetColorAndOpacity (Variables|/Game/MyGame/UI/WB_UI.WB_UI_C|GetQuest1 (Variables|/Game/MyGame/UI/MyHUD.MyHUD_C|GetUI_Ref _asmy_hud)) (Utilities|Struct|MakeSlateColor "(R=0.000000,G=1.000000,B=0.171535,A=1.000000)"))
              (Variables|/Script/UMG.TextBlock|SetText (Variables|/Game/MyGame/UI/WB_UI.WB_UI_C|GetQuest2 (Variables|/Game/MyGame/UI/MyHUD.MyHUD_C|GetUI_Ref _asmy_hud)) "Talk to the mysterious man"))))))))

(event EventStartDialogue
  (bind _dialogue1 (Variables|Default|GetDialogue1))
  (bind _dialogue2 (Variables|Default|GetDialogue2))
  (if (not (Utilities|IsValid (Variables|Default|GetDialogueWidget)))
    (bind _returnvalue (UserInterface|CreateWidget "/Game/MyGame/UI/WB_Dialogue.WB_Dialogue_C"))
    (bind _output_get (Variables|Default|SetDialogueWidget _returnvalue))
    (UserInterface|Viewport|AddtoViewport _output_get 0)
    (bind _asbp_player (Utilities|Casting|CastToBP_Player (Game|Player|GetPlayerPawn 0)))
    (Default|DisableMovement _asbp_player)
    (else
      (switch int (Variables|Default|GetEventIndex)
        (:0
          (Variables|/Script/UMG.TextBlock|SetText (Variables|/Game/MyGame/UI/WB_Dialogue.WB_Dialogue_C|GetDialogueText (Variables|Default|GetDialogueWidget)) (Utilities|Text|ToText(String) (Utilities|Array|Get(acopy) _dialogue1 (Variables|Default|GetDialogueIndex))))
          (Math|Integer|IncrementInt (Variables|Default|GetDialogueIndex)
            (:%20%20
              (if (> (Variables|Default|GetDialogueIndex) (Utilities|Array|Length _dialogue1))
                (Widget|RemovefromParent (Variables|Default|GetDialogueWidget) :!label _label)
                (bind _asbp_player_2 (Utilities|Casting|CastToBP_Player (Game|Player|GetPlayerPawn 0))
                  (:then
                    (Default|EnableMovement _asbp_player_2)
                    (Variables|Default|SetDialogueIndex 0)
                    (Variables|Default|SetDialogueWidget 0)
                    (bind _asmy_hud (Utilities|Casting|CastToMyHUD (HUD|GetHUD (Game|GetPlayerController 0))))
                    (switch int (Variables|Default|GetEventIndex)
                      (:0
                        (Variables|/Script/UMG.TextBlock|SetText (Variables|/Game/MyGame/UI/WB_UI.WB_UI_C|GetQuest1 (Variables|/Game/MyGame/UI/MyHUD.MyHUD_C|GetUI_Ref _asmy_hud)) "Collect the plants the mysterious man asked for (0/10)")
                        (Variables|/Script/UMG.TextBlock|SetText (Variables|/Game/MyGame/UI/WB_UI.WB_UI_C|GetQuest2 (Variables|/Game/MyGame/UI/MyHUD.MyHUD_C|GetUI_Ref _asmy_hud)) "")
                        (Variables|Default|SetEventIndex 1))
                      (:2
                        (Variables|/Script/UMG.TextBlock|SetText (Variables|/Game/MyGame/UI/WB_UI.WB_UI_C|GetQuest1 (Variables|/Game/MyGame/UI/MyHUD.MyHUD_C|GetUI_Ref _asmy_hud)) "Season 1 Complete! Wait for Season 2 :)")
                        (Variables|/Script/UMG.TextBlock|SetText (Variables|/Game/MyGame/UI/WB_UI.WB_UI_C|GetQuest2 (Variables|/Game/MyGame/UI/MyHUD.MyHUD_C|GetUI_Ref _asmy_hud)) "")
                        (Variables|Default|SetEventIndex 3))))
                  (:CastFailed
                    (Development|PrintString "Cast Failed lol")))))))
        (:2
          (Variables|/Script/UMG.TextBlock|SetText (Variables|/Game/MyGame/UI/WB_Dialogue.WB_Dialogue_C|GetDialogueText (Variables|Default|GetDialogueWidget)) (Utilities|Text|ToText(String) (Utilities|Array|Get(acopy) _dialogue2 (Variables|Default|GetDialogueIndex))))
          (Math|Integer|IncrementInt (Variables|Default|GetDialogueIndex)
            (:%20%20
              (if (> (Variables|Default|GetDialogueIndex) (Utilities|Array|Length _dialogue2))
                (goto _label)))))))))

(fn ConstructionScript)